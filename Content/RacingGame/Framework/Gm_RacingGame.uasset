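; Game mode for a timed checkpoint race, won by crossing the finish line before time runs out.
; BeginPlay binds to every BP_Checkpoint, separating finish from timed checkpoints, then enters a print-only pre-race state.
; StartCountdown, not called here, delays before starting the lose timer, which checkpoints extend by re-setting it with added time and a HUD animation.
; Finishing stops the vehicle and disables input; winning also shows a win screen.
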(event `self.ReceiveBeginPlay`
  (`|ExecutionSequence`
    (:`then_0`
      (bind _outactors (`GameplayStatics.GetAllActorsOfClass` "/Game/RacingGame/Checkpoints/BP_Checkpoint.BP_Checkpoint_C"))
      (for _array_element _outactors
        (if (`/Game/RacingGame/Checkpoints/BP_Checkpoint.isFinishLine` _array_element)
          (add `/Game/RacingGame/Checkpoints/BP_Checkpoint.OnCheckpointCrossed` _array_element (`|CreateDelegate` :!event `Win_CrossTheFinishLine`))
          (else
            (add `/Game/RacingGame/Checkpoints/BP_Checkpoint.OnCheckpointCrossedWithTime` _array_element (`|CreateDelegate` :!event `CrossedACheckpoint`))))))
    (:`then_1`
      (`self.PreRace`))))

(event `PreRace`
  (`KismetSystemLibrary.PrintText` "In Pre Race State"))

(event `Start Countdown`
  (`KismetSystemLibrary.PrintText` "Start Countdown")
  (`KismetSystemLibrary.Delay` (`self.Coutdown Duration`))
  (`self.Game Start`))

(event `Game Start`
  (`KismetSystemLibrary.PrintText` "Game Start")
  (bind _returnvalue (`KismetSystemLibrary.K2_SetTimerDelegate` (delegate `Lose?OutOfTime`) (`self.Start Timer Duration`)))
  (set `self.Time Remaining Timer` _returnvalue))

(event `Lose?OutOfTime`
  (`self.Game Finish` false))

(event `Win_CrossTheFinishLine`
  (`KismetSystemLibrary.K2_ClearAndInvalidateTimerHandle` (`self.Time Remaining Timer`))
  (bind _returnvalue (`|CreateWidget` "/Game/RacingGame/UI/WBP_WinScreen.WBP_WinScreen_C"))
  (`UserWidget.AddToViewport` _returnvalue 0)
  (set `PlayerController.bShowMouseCursor` true (`GameplayStatics.GetPlayerController` 0))
  (`self.Game Finish` true))

(event `Game Finish`
  (params (Win :type Boolean))
  (bind _returnvalue (`GameplayStatics.GetPlayerPawn` 0))
  (`KismetSystemLibrary.PrintText` (select `bool` Win :`false` "You lose" :`true` "You Win" :!type "Text"))
  (`self.DisableInput` _returnvalue (`GameplayStatics.GetPlayerController` 0))
  (bind _aswheeled_vehicle_pawn (cast `WheeledVehiclePawn` _returnvalue))
  (bind _vehiclemovementcomponent (`WheeledVehiclePawn.VehicleMovementComponent` _aswheeled_vehicle_pawn))
  (`ChaosVehicleMovementComponent.SetThrottleInput` _vehiclemovementcomponent 0.0)
  (`ChaosVehicleMovementComponent.SetHandbrakeInput` _vehiclemovementcomponent true)
  (`ChaosVehicleMovementComponent.SetSteeringInput` _vehiclemovementcomponent 1.0))

(event `CrossedACheckpoint`
  (params (TimeToAdd :type Integer))
  (`self.AddTimeToTimer` TimeToAdd))

(fn `AddTimeToTimer`
  (params (TimeToAdd :type Integer))
  (bind _returnvalue (`KismetSystemLibrary.K2_SetTimerDelegate` (`|CreateDelegate` :!event `Lose?OutOfTime`) (+ (`KismetSystemLibrary.K2_GetTimerRemainingTimeHandle` (`self.Time Remaining Timer`)) (`local.TimeToAdd`))))
  (set `self.Time Remaining Timer` _returnvalue)
  (bind _asvehicle_player_controller (cast `/Game/VehicleTemplate/Blueprints/VehiclePlayerController` (`GameplayStatics.GetPlayerController` 0)))
  (`/Game/VehicleTemplate/Blueprints/VehicleUI.PlayAddedTimeAnim` (`/Game/VehicleTemplate/Blueprints/VehiclePlayerController.VehicleHud` _asvehicle_player_controller)))

(fn `UserConstructionScript`)